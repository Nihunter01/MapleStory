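; BP_EnemyBase is a base enemy Blueprint that switches a Paper2D sprite between idle and move animations.
; MovementState forwards a moving flag to a server event, which stores it in BisMoving.
; The flag's RepNotify sets the sprite's flipbook from the idle or move animation in AnimalInfo, keeping animation in sync across the network.
; GetEnemyRef returns the enemy itself.
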(event `/Game/BluePrints/Interfaces/INT_EnemyController.MovementState`
  (params (bisMoving :type Boolean))
  (`self.SRV_MovementState` bisMoving))

(event `SRV_MovementState`
  (params (bisMoving :type Boolean))
  (set `self.bisMoving` bisMoving))

(fn `GetEnemyRef`
  (returns (Enemy :type "/Game/BluePrints/Enemy/BP_EnemyBase Object Reference"))
  (return self))

(fn `OnRep_BisMoving`
  (bind _sprite (`self.Sprite`))
  (bind (_idleanimation _moveanimation) (break `/Game/BluePrints/Structs/ST_AnimalInfo` (`self.AnimalInfo`)))
  (if (not (`self.bisMoving`))
    (`PaperFlipbookComponent.SetFlipbook` _sprite _idleanimation)
    (else
      (`PaperFlipbookComponent.SetFlipbook` _sprite _moveanimation))))

(fn `UserConstructionScript`
  (`parent.UserConstructionScript`))