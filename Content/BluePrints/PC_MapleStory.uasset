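; Player controller for a MapleStory-style game that handles character selection, spawning and possession.
; On BeginPlay it shows the character selection widget through a client-prefixed event.
; Selection passes through a server-prefixed event to the GameMode, requesting a spawn via interface-style messages.
; SpawnPlayer spawns the given character class, adjusting for collisions but always spawning, then possesses it.
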(event `self.ReceiveBeginPlay`
  (`self.InitializeWidgets`))

(event `/Game/BluePrints/Interfaces/INT_PlayerController.InitializeWidgets`
  (`self.CL_InitializeWidgets`))

(event `CL_InitializeWidgets`
  (bind _returnvalue (`|CreateWidget` "/Game/BluePrints/UI/WB_CharacterSelection.WB_CharacterSelection_C"))
  (bind _output_get (set `self.WB_ChracterSelection` _returnvalue))
  (`UserWidget.AddToViewport` _output_get 0))

(event `/Game/BluePrints/Interfaces/INT_PlayerController.SelectCharacter`
  (params (Player :type "Actor Class Reference") (SpawnLocation :type "Vector Structure"))
  (`self.SRV_SelectCharacter` Player SpawnLocation))

(event `SRV_SelectCharacter`
  (params (Player :type "Actor Class Reference") (SpawnLocation :type "Vector Structure"))
  (bind _gamemode (message `/Game/BluePrints/Interfaces/INT_GameMode.GetGameModeRef` (`GameplayStatics.GetGameMode`)))
  (message `/Game/BluePrints/Interfaces/INT_GameMode.RequestSpawnPlayer` _gamemode self Player SpawnLocation))

(event `/Game/BluePrints/Interfaces/INT_PlayerController.SpawnPlayer`
  (params (Player :type "Actor Class Reference") (SpawnTransform :type "Transform Structure"))
  (bind _returnvalue (`|SpawnActorFromClass` Player SpawnTransform "AdjustIfPossibleButAlwaysSpawn" "MultiplyWithRoot" null null))
  (bind _playerbase (message `/Game/BluePrints/Interfaces/INI_PlayerBase.GetPlayerRef` _returnvalue))
  (`self.Possess` _playerbase))

(fn `GetPlayerControllerRef`
  (returns (PlayerController :type "/Game/BluePrints/PC_MapleStory Object Reference"))
  (return self))

(fn `UserConstructionScript`)